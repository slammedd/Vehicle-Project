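; Neon sign Blueprint for "The Hole" that randomly flickers two material slots on its static mesh.
; BeginPlay calls FlickerMain, then FlickerSecond; each waits a fixed delay, then on a coin flip briefly swaps its slot to a flicker material.
; FlickerMain loops by calling itself after either outcome.
; FlickerSecond repeats only after a flicker; its no-flicker branch calls FlickerMain instead, ending the second slot's loop.
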(event `self.ReceiveBeginPlay`
  (`self.Flicker Main`)
  (`self.Flicker Second`))

(event `Flicker Main`
  (bind _staticmesh (`self.StaticMesh`))
  (`KismetSystemLibrary.Delay` 7.5)
  (if (== (`KismetMathLibrary.RandomIntegerInRange` 0 1) 0)
    (`PrimitiveComponent.SetMaterial` _staticmesh 1 "/Game/Materials/MAT_Neon_Flicker_hole.MAT_Neon_Flicker_hole")
    (`KismetSystemLibrary.Delay` (`KismetMathLibrary.RandomFloatInRange` 0.1 0.9))
    (`PrimitiveComponent.SetMaterial` _staticmesh 1 "/Game/Materials/MAT_Neon_Normal_hole.MAT_Neon_Normal_hole")
    (`self.Flicker Main`)
    (else
      (`self.Flicker Main`))))

(event `Flicker Second`
  (bind _staticmesh (`self.StaticMesh`))
  (`KismetSystemLibrary.Delay` 7.5)
  (if (== (`KismetMathLibrary.RandomIntegerInRange` 0 1) 0)
    (`PrimitiveComponent.SetMaterial` _staticmesh 2 "/Game/Materials/MAT_Neon_Flicker_hole1.MAT_Neon_Flicker_hole1")
    (`KismetSystemLibrary.Delay` (`KismetMathLibrary.RandomFloatInRange` 0.1 0.9))
    (`PrimitiveComponent.SetMaterial` _staticmesh 2 "/Game/Materials/MAT_Neon_Normal_hole1.MAT_Neon_Normal_hole1")
    (`self.Flicker Second`)
    (else
      (`self.Flicker Main`))))

(fn `UserConstructionScript`)
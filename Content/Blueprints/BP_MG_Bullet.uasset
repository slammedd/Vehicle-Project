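; Machine gun bullet that damages enemies on hit, with distance falloff and random critical hits.
; A looping timer randomly erodes damage from spawn until impact, and a critical chance rolled at BeginPlay multiplies what remains.
; Hits damage BPI_Enemy actors through the interface and spawn a damage number, with non-critical opacity scaled by remaining damage.
; Each impact plays particles and sound chosen by physical surface type, then destroys the bullet.
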(event `self.ReceiveBeginPlay`
  (set `self.Damage` (`self.Base Damage`))
  ;[1 1 1] Distance Damage Decay
  (bind _returnvalue (`KismetSystemLibrary.K2_SetTimerDelegate` (delegate `Damage Distance Decay`) 0.01 true))
  (set `self.Damage Decay Timer` _returnvalue)
  ;[1 1 1] Critical Hit Chance
  (if (== (`KismetMathLibrary.RandomIntegerInRange` 0 19) 0)
    (set `self.Critical Hit` true)
    (else
      (set `self.Critical Hit` false))))

(event `Damage Distance Decay`
  ;[1 1 1] Distance Damage Decay
  (set `self.Damage` (- (`self.Damage`) (`KismetMathLibrary.RandomFloatInRange` 1.0 2.0))))

(event `self.StaticMesh.OnComponentHit`
  (params (HitComponent :type "PrimitiveComponent Object Reference") (OtherActor :type "Actor Object Reference") (OtherComp :type "PrimitiveComponent Object Reference") (NormalImpulse :type "Vector Structure") (Hit :type "HitResult Structure (by ref)"))
  (bind (_bblockinghit _binitialoverlap _time _distance _location _impactpoint _normal _impactnormal _physmat) (`GameplayStatics.BreakHitResult` Hit))
  (`KismetSystemLibrary.K2_ClearAndInvalidateTimerHandle` (`self.Damage Decay Timer`))
  (if (`KismetSystemLibrary.DoesImplementInterface` OtherActor "/Game/Blueprints/BPI_Enemy.BPI_Enemy_C")
    (if (`self.Critical Hit`)
      (message `/Game/Blueprints/BPI_Enemy.Damage Enemy` OtherActor (* (`self.Damage`) 5.0))
      (bind _returnvalue (`|SpawnActorFromClass` "/Game/Blueprints/BP_Damage_Number.BP_Damage_Number_C" (`KismetMathLibrary.MakeTransform` _impactpoint) "AdjustIfPossibleButAlwaysSpawn" "MultiplyWithRoot" null null))
      (`/Game/Blueprints/BP_Damage_Number.Damage Detail Pass Through` _returnvalue 1.0 (* (`self.Damage`) 5.0) (`self.Critical Hit`))
      (else
        (message `/Game/Blueprints/BPI_Enemy.Damage Enemy` OtherActor (`self.Damage`))
        (bind _returnvalue_2 (`|SpawnActorFromClass` "/Game/Blueprints/BP_Damage_Number.BP_Damage_Number_C" (`KismetMathLibrary.MakeTransform` _impactpoint) "AdjustIfPossibleButAlwaysSpawn" "MultiplyWithRoot" null null))
        (bind _damage_opacity (`self.Calculate Damage Opacity`))
        (`/Game/Blueprints/BP_Damage_Number.Damage Detail Pass Through` _returnvalue_2 _damage_opacity (`self.Damage`) (`self.Critical Hit`)))))
  (switch `EPhysicalSurface` (`PhysicalMaterial.SurfaceType` _physmat)
    (:`SurfaceType_Default`
      (`GameplayStatics.SpawnEmitterAtLocation` "/Game/Realistic_Starter_VFX_Pack_Vol2/Particles/Hit/P_Ceramic.P_Ceramic" _impactpoint)
      (`GameplayStatics.PlaySoundAtLocation` "/Game/Audio/Impacts/SC_Concrete_Bullet_Impact.SC_Concrete_Bullet_Impact" _impactpoint (struct) 1.0 1.0 0.0 null null null null :!label _label))
    (:`SurfaceType1`
      (`GameplayStatics.SpawnEmitterAtLocation` "/Game/Realistic_Starter_VFX_Pack_Vol2/Particles/Hit/P_Default.P_Default" _impactpoint)
      (`GameplayStatics.PlaySoundAtLocation` "/Game/Audio/Impacts/SC_Metal_Bullet_Impact.SC_Metal_Bullet_Impact" _impactpoint (struct) 1.0 1.0 0.0 null null null null))
    (:`SurfaceType2`
      (`GameplayStatics.SpawnEmitterAtLocation` "/Game/Realistic_Starter_VFX_Pack_Vol2/Particles/Hit/P_Brick.P_Brick" _impactpoint)
      (goto _label))
    (:`SurfaceType3`
      (`GameplayStatics.SpawnEmitterAtLocation` "/Game/Realistic_Starter_VFX_Pack_Vol2/Particles/Hit/P_Concrete.P_Concrete" _impactpoint)
      (goto _label))
    (:`SurfaceType4`
      (`GameplayStatics.SpawnEmitterAtLocation` "/Game/Realistic_Starter_VFX_Pack_Vol2/Particles/Hit/P_Ice.P_Ice" _impactpoint)
      (`GameplayStatics.PlaySoundAtLocation` "/Game/Audio/Impacts/SC_Glass_Bullet_Impact.SC_Glass_Bullet_Impact" _impactpoint (struct) 1.0 1.0 0.0 null null null null)))
  (`self.K2_DestroyActor`))

(fn `Calculate Damage Opacity`
  (returns (`Damage Opacity` :type "Float (double-precision)"))
  (return (`KismetMathLibrary.NormalizeToRange` (`self.Damage`) 0.0 (`self.Base Damage`))))

(fn `UserConstructionScript`)
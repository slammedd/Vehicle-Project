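; Neon "Clothe It" shop sign actor that randomly flickers during play.
; A self-calling Flicker event starts on BeginPlay, waits a fixed interval, then has a coin-flip chance to briefly swap one static mesh material slot to a flicker material instance.
; After a random short delay it restores the normal neon material and loops again.
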(event `self.ReceiveBeginPlay`
  (`self.Flicker`))

(event `Flicker`
  (bind _staticmesh (`self.StaticMesh`))
  (`KismetSystemLibrary.Delay` 7.5)
  (if (== (`KismetMathLibrary.RandomIntegerInRange` 0 1) 0)
    (`PrimitiveComponent.SetMaterial` _staticmesh 1 "/Game/Materials/MAT_Neon_Flicker_Inst1.MAT_Neon_Flicker_Inst1")
    (`KismetSystemLibrary.Delay` (`KismetMathLibrary.RandomFloatInRange` 0.1 0.9))
    (`PrimitiveComponent.SetMaterial` _staticmesh 1 "/Game/Materials/MAT_Neon_Normal_clothe.MAT_Neon_Normal_clothe")
    (`self.Flicker`)
    (else
      (`self.Flicker`))))

(fn `UserConstructionScript`)
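; BP_Mini_Rocket is a homing rocket that explodes on hit or after ten seconds, damaging an enemy within its blast radius.
; Homing targets the last BPI_Enemy actor found at spawn.
; A looping timer randomly decays damage during flight, and a spawn-time roll can make it a critical hit with multiplied damage.
; A sphere trace with DoOnce damages one enemy and spawns a damage number, faded by remaining damage on non-crits.
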(event `self.ReceiveBeginPlay`
  (bind _returnvalue (`self.K2_GetActorLocation`))
  (set `self.Base Damage` (`self.Damage`))
  (bind _returnvalue_2 (`KismetSystemLibrary.K2_SetTimerDelegate` (delegate `Damage Distance Decay`) 0.01 true))
  (set `self.Damage Decay Timer` _returnvalue_2)
  (if (== (`KismetMathLibrary.RandomIntegerInRange` 0 19) 0)
    (set `self.Critical Hit` true)
    (else
      (set `self.Critical Hit` false)))
  (bind _outactors (`GameplayStatics.GetAllActorsWithInterface` "/Game/Blueprints/BPI_Enemy.BPI_Enemy_C"))
  (for _array_element _outactors
    (set `ProjectileMovementComponent.HomingTargetComponent` (`Actor.RootComponent` _array_element) (`self.ProjectileMovement`)))
  (`KismetSystemLibrary.Delay` 10.0)
  (`KismetSystemLibrary.K2_ClearAndInvalidateTimerHandle` (`self.Damage Decay Timer`) :!label _label)
  (`GameplayStatics.SpawnEmitterAtLocation` "/Game/Realistic_Starter_VFX_Pack_Vol2/Particles/Explosion/P_Explosion_Big_A.P_Explosion_Big_A" (`self.K2_GetActorLocation`))
  (`GameplayStatics.PlaySoundAtLocation` "/Game/Audio/SC_Missile_Explosion.SC_Missile_Explosion" _returnvalue (struct) 1.0 1.0 0.0 null null null null)
  (bind _outhits (`KismetSystemLibrary.SphereTraceMulti` _returnvalue _returnvalue 350.0 "TraceTypeQuery1"))
  (for _array_element_2 _outhits
    (bind (_bblockinghit _binitialoverlap _time _distance _location _impactpoint _normal _impactnormal _physmat _hitactor) (`GameplayStatics.BreakHitResult` _array_element_2))
    (if (`KismetSystemLibrary.DoesImplementInterface` _hitactor "/Game/Blueprints/BPI_Enemy.BPI_Enemy_C")
      (`/Engine/EditorBlueprintResources/StandardMacros.DoOnce` false
        (:`Completed`
          (if (`self.Critical Hit`)
            (message `/Game/Blueprints/BPI_Enemy.Damage Enemy` _hitactor (* (`self.Damage`) 5.0))
            (bind _returnvalue_3 (`|SpawnActorFromClass` "/Game/Blueprints/BP_Damage_Number.BP_Damage_Number_C" (`KismetMathLibrary.MakeTransform` (`self.K2_GetActorLocation`)) "AdjustIfPossibleButAlwaysSpawn" "MultiplyWithRoot" null null))
            (`/Game/Blueprints/BP_Damage_Number.Damage Detail Pass Through` _returnvalue_3 1.0 (* (`self.Damage`) 5.0) (`self.Critical Hit`))
            (else
              (message `/Game/Blueprints/BPI_Enemy.Damage Enemy` _hitactor (`self.Damage`))
              (bind _returnvalue_4 (`|SpawnActorFromClass` "/Game/Blueprints/BP_Damage_Number.BP_Damage_Number_C" (`KismetMathLibrary.MakeTransform` (`self.K2_GetActorLocation`)) "AdjustIfPossibleButAlwaysSpawn" "MultiplyWithRoot" null null))
              (bind _damage_opacity (`self.Calculate Damage Opacity`))
              (`/Game/Blueprints/BP_Damage_Number.Damage Detail Pass Through` _returnvalue_4 _damage_opacity (`self.Damage`) (`self.Critical Hit`))))))))
  (`self.K2_DestroyActor`))

(event `Damage Distance Decay`
  (set `self.Damage` (- (`self.Damage`) (`KismetMathLibrary.RandomFloatInRange` 1.0 2.0))))

(event `self.StaticMesh.OnComponentHit`
  (params (HitComponent :type "PrimitiveComponent Object Reference") (OtherActor :type "Actor Object Reference") (OtherComp :type "PrimitiveComponent Object Reference") (NormalImpulse :type "Vector Structure") (Hit :type "HitResult Structure (by ref)"))
  (`/Engine/EditorBlueprintResources/StandardMacros.DoOnce` false
    (:`Completed`
      (goto _label))))

(fn `Calculate Damage Opacity`
  (returns (`Damage Opacity` :type "Float (double-precision)"))
  (return (`KismetMathLibrary.NormalizeToRange` (`self.Damage`) 0.0 (`self.Base Damage`))))

(fn `UserConstructionScript`)
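; BP_Damage_Number is an actor that displays a damage number as a short-lived, physics-launched popup.
; On BeginPlay it gives its Cube component a random upward and sideways velocity-change impulse, then destroys itself after a fixed delay.
; DamageDetailPassThrough forwards opacity, damage value and critical-hit data to the WB_Damage_Number widget held by its Widget component.
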(event `self.ReceiveBeginPlay`
  (`PrimitiveComponent.AddImpulse` (`self.Cube`) (`KismetMathLibrary.MakeVector` (`KismetMathLibrary.RandomFloatInRange` -400.0 400.0) (`KismetMathLibrary.RandomFloatInRange` -400.0 400.0) (`KismetMathLibrary.RandomFloatInRange` 400.0 650.0)) "None" true)
  (`KismetSystemLibrary.Delay` 3.5)
  (`self.K2_DestroyActor`))

(fn `Damage Detail Pass Through`
  (params (`Damage Opacity` :type "Float (double-precision)") (`Damage Number` :type "Float (double-precision)") (`Critical Hit` :type Boolean))
  (bind _aswb_damage_number (cast `/Game/UI/WB_Damage_Number` (`WidgetComponent.GetWidget` (`self.Widget`))))
  (`/Game/UI/WB_Damage_Number.Pass Damage Details` _aswb_damage_number `Damage Opacity` `Damage Number` `Critical Hit`))

(fn `UserConstructionScript`)
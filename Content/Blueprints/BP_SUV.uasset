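; Player-driven Chaos wheeled SUV that takes Enhanced Input for throttle, brake, steering, handbrake, horn and respawn.
; BeginPlay creates the HUD and dynamic body material, whose emissive brake lights fade via timeline.
; Tick reads engine RPM and MPH speed, driving engine audio and Niagara exhaust smoke from RPM.
; Reset, also run at BeginPlay, lifts the car and levels it keeping yaw, only when nearly stationary.
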(event `self.ReceiveTick`
  (params (DeltaSeconds :type "Float (single-precision)"))
  (`self.Engine Sounds`)
  (`self.Read RPM`)
  (`self.Exhaust Smoke RPM Control`)
  (`self.Read Speed MPH`))

(event `self.ReceiveBeginPlay`
  ;[1 1 1] Initialise Input
  (bind _asplayer_controller (cast `PlayerController` (`self.GetController`)))
  (`EnhancedInputSubsystemInterface.AddMappingContext` (pcsubsystem `EnhancedInputLocalPlayerSubsystem` _asplayer_controller) "/Game/Input/IMC_Default.IMC_Default" 0 (struct))
  ;[1 1 1] Initialise ChaosWheeledVehicleComponent Reference
  (bind _aschaos_wheeled_vehicle_movement_component (cast `ChaosWheeledVehicleMovementComponent` (`self.VehicleMovementComponent`)))
  (set `self.Chaos Wheeled Vehicle Movement Component` _aschaos_wheeled_vehicle_movement_component)
  ;[1 1 1] Initialise HUD
  (bind _returnvalue (`|CreateWidget` "/Game/UI/WB_HUD.WB_HUD_C"))
  (bind _output_get (set `self.HUD` _returnvalue))
  (`UserWidget.AddToViewport` _output_get 0)
  ;[1 1 1] Initialise Material
  (bind _returnvalue_2 (`PrimitiveComponent.CreateDynamicMaterialInstance` (`self.Mesh`) 2 null "None"))
  (set `self.Body Material` _returnvalue_2)
  (`self.Reset Car`))

(event `Read RPM`
  ;[1 1 1] Read RPM
  (set `self.Engine RPM` (`ChaosWheeledVehicleMovementComponent.GetEngineRotationSpeed` (`self.Chaos Wheeled Vehicle Movement Component`))))

(event `Read Speed MPH`
  ;[1 1 1] Calculate Speed in MPH
  (set `self.Speed MPH` (* (`KismetMathLibrary.VSize` (`self.GetVelocity`)) 0.0224)))

(event `Engine Sounds`
  (bind _sc_suv_engine (`self.SC_SUV_Engine`))
  (bind _returnvalue (`ChaosWheeledVehicleMovementComponent.GetEngineRotationSpeed` (`self.Chaos Wheeled Vehicle Movement Component`)))
  ;[1 1 1] Engine Sounds
  (if (< _returnvalue 600.0)
    (`AudioParameterControllerInterface.SetFloatParameter` _sc_suv_engine "RPM" 600.0)
    (else
      (`AudioParameterControllerInterface.SetFloatParameter` _sc_suv_engine "RPM" _returnvalue))))

(event `EnhancedInput|/Game/Input/IA_Handbrake`
  (params (ActionValue :type Boolean) (ElapsedSeconds :type "Float (double-precision)") (TriggeredSeconds :type "Float (double-precision)") (InputAction :type "InputAction Object Reference" :default "/Game/Input/IA_Handbrake.IA_Handbrake"))
  (bind _returnvalue (`self.K2_GetActorLocation`))
  (bind _vehiclemovementcomponent (`self.VehicleMovementComponent`))
  ;[1 1 1] Vehicle Movement
  (:`Triggered`
    (`ChaosVehicleMovementComponent.SetHandbrakeInput` _vehiclemovementcomponent true)
    ;[1 1 1] Handbrake Sound
    (`/Engine/EditorBlueprintResources/StandardMacros.DoOnce` false :!label _label
      (:`Completed`
        (`GameplayStatics.PlaySoundAtLocation` "/Game/Audio/SC_Handbrake_On.SC_Handbrake_On" _returnvalue (struct) 1.0 1.0 0.0 null null null null))))
  (:`Canceled`
    (`ChaosVehicleMovementComponent.SetHandbrakeInput` _vehiclemovementcomponent false :!label _label_2)
    (`GameplayStatics.PlaySoundAtLocation` "/Game/Audio/SC_Handbrake_Off.SC_Handbrake_Off" _returnvalue (struct) 1.0 1.0 0.0 null null null null)
    (goto _label :!via `Reset`))
  (:`Completed`
    (goto _label_2)))

(event `EnhancedInput|/Game/Input/IA_Throttle`
  (params (ActionValue :type "Float (double-precision)") (ElapsedSeconds :type "Float (double-precision)") (TriggeredSeconds :type "Float (double-precision)") (InputAction :type "InputAction Object Reference" :default "/Game/Input/IA_Throttle.IA_Throttle"))
  (bind _vehiclemovementcomponent (`self.VehicleMovementComponent`))
  ;[1 1 1] Vehicle Movement
  (:`Triggered`
    (`ChaosVehicleMovementComponent.SetThrottleInput` _vehiclemovementcomponent ActionValue))
  (:`Canceled`
    (`ChaosVehicleMovementComponent.SetThrottleInput` _vehiclemovementcomponent 0.0 :!label _label_3))
  (:`Completed`
    (goto _label_3)))

(event `EnhancedInput|/Game/Input/IA_Brake`
  (params (ActionValue :type "Float (double-precision)") (ElapsedSeconds :type "Float (double-precision)") (TriggeredSeconds :type "Float (double-precision)") (InputAction :type "InputAction Object Reference" :default "/Game/Input/IA_Brake.IA_Brake"))
  (bind _vehiclemovementcomponent (`self.VehicleMovementComponent`))
  ;[1 1 1] Vehicle Movement
  (:`Triggered`
    (`ChaosVehicleMovementComponent.SetBrakeInput` _vehiclemovementcomponent ActionValue)
    ;[1 1 1] Brake Lights
    (`/Engine/EditorBlueprintResources/StandardMacros.DoOnce` false :!label _label_4
      (:`Completed`
        (bind (_direction _emissive_power) (`Timeline|Brake Lights` :!label _label_5)
          (:`Update`
            (`MaterialInstanceDynamic.SetScalarParameterValue` (`self.Body Material`) "Emissive Power" _emissive_power))))))
  (:`Canceled`
    (`ChaosVehicleMovementComponent.SetBrakeInput` _vehiclemovementcomponent 0.0 :!label _label_6)
    (`|ExecutionSequence`
      (:`then_0`
        (goto _label_4 :!via `Reset`))
      (:`then_1`
        (goto _label_5 :!via `Reverse`))))
  (:`Completed`
    (goto _label_6)))

(event `Reset Car`
  (bind (_returnvalue_roll _returnvalue_pitch _returnvalue_yaw) (`KismetMathLibrary.BreakRotator` (`self.K2_GetActorRotation`)))
  ;[1 1 1] Random Spawn Location
  (if (<= (`self.Speed MPH`) 5.0)
    (`self.K2_SetActorLocation` (+ (`self.K2_GetActorLocation`) (0.0 0.0 500.0)) true true)
    (`self.K2_SetActorRotation` (`KismetMathLibrary.MakeRotator` 0.0 0.0 _returnvalue_yaw) true)
    (else
      (`KismetSystemLibrary.PrintString` "CANT RESET WHILE MOVING" true true (struct :`R` 1.0 :`A` 1.0)))))

(event `EnhancedInput|/Game/Input/IA_Steering`
  (params (ActionValue :type "Float (double-precision)") (ElapsedSeconds :type "Float (double-precision)") (TriggeredSeconds :type "Float (double-precision)") (InputAction :type "InputAction Object Reference" :default "/Game/Input/IA_Steering.IA_Steering"))
  (bind _vehiclemovementcomponent (`self.VehicleMovementComponent`))
  ;[1 1 1] Vehicle Movement
  (:`Triggered`
    (`ChaosVehicleMovementComponent.SetSteeringInput` _vehiclemovementcomponent ActionValue))
  (:`Canceled`
    (`ChaosVehicleMovementComponent.SetSteeringInput` _vehiclemovementcomponent 0.0 :!label _label_7))
  (:`Completed`
    (goto _label_7)))

(event `EnhancedInput|/Game/Input/IA_Respawn`
  (params (ActionValue :type Boolean) (ElapsedSeconds :type "Float (double-precision)") (TriggeredSeconds :type "Float (double-precision)") (InputAction :type "InputAction Object Reference" :default "/Game/Input/IA_Respawn.IA_Respawn"))
  (:`Triggered`
    (`self.Reset Car`)))

(event `Exhaust Smoke RPM Control`
  ;[1 1 1] Exhaust Smoke
  (`NiagaraComponent.SetVariableFloat` (`self.Exhaust Smoke`) "RPM Spawn Rate" (`KismetMathLibrary.FClamp` (* (`self.Engine RPM`) 0.1) 8.0 500.0))
  (`NiagaraComponent.SetVariableFloat` (`self.Exhaust Smoke`) "RPM Velocity" (`KismetMathLibrary.FClamp` (* (`self.Engine RPM`) 0.1) 150.0 1500.0)))

(event `EnhancedInput|/Game/Input/IA_Horn`
  (params (ActionValue :type Boolean) (ElapsedSeconds :type "Float (double-precision)") (TriggeredSeconds :type "Float (double-precision)") (InputAction :type "InputAction Object Reference" :default "/Game/Input/IA_Horn.IA_Horn"))
  ;[1 1 1] Horn Sound
  (:`Triggered`
    (`/Engine/EditorBlueprintResources/StandardMacros.DoOnce` false :!label _label_8
      (:`Completed`
        (`GameplayStatics.PlaySoundAtLocation` "/Game/Audio/SC_Horn.SC_Horn" (`self.K2_GetActorLocation`) (struct) 1.0 1.0 0.0 null null null null))))
  (:`Canceled`
    (goto _label_8 :!via `Reset`))
  (:`Completed`
    (goto _label_8 :!via `Reset`)))

(fn `UserConstructionScript`)